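; Main game mode that fades sun and sky light intensity with the BP_GoodSky time of day.
; BeginPlay caches the first sky, directional light and skylight actors found in the level.
; Tick offsets the sky's time by 12 hours, ramping both lights up in the morning and down in the evening, leaving them untouched otherwise.
; SetHowLongDay passes a day length in minutes to the sky.
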(event `self.ReceiveBeginPlay`
  (bind _outactors (`GameplayStatics.GetAllActorsOfClass` "/Game/OriginalContents/GoodSky/Blueprint/BP_GoodSky.BP_GoodSky_C"))
  (set `self.Sky` (`|GetArrayItem` _outactors))
  (bind _outactors_2 (`GameplayStatics.GetAllActorsOfClass` "/Script/Engine.DirectionalLight"))
  (set `self.SunLight` (`|GetArrayItem` _outactors_2))
  (bind _outactors_3 (`GameplayStatics.GetAllActorsOfClass` "/Script/Engine.SkyLight"))
  (set `self.SkyLight` (`|GetArrayItem` _outactors_3)))

(event `self.ReceiveTick`
  (params (DeltaSeconds :type "Float (single-precision)"))
  (bind _lightcomponent (`Light.LightComponent` (`self.SunLight`)))
  (bind _lightcomponent_2 (`SkyLight.LightComponent` (`self.SkyLight`)))
  (bind _output_get (set `self.CurrentTime` (mod (+ (`/Game/OriginalContents/GoodSky/Blueprint/BP_GoodSky.Get Rotator To Time of Day` (`self.Sky`)) 12.0) 24.0)))
  (if (`KismetMathLibrary.InRange_FloatFloat` _output_get 6.0 10.0)
    (`LightComponent.SetIntensity` _lightcomponent (`KismetMathLibrary.MapRangeClamped` _output_get 6.0 10.0 0.0 10.0))
    (`SkyLightComponent.SetIntensity` _lightcomponent_2 (`KismetMathLibrary.MapRangeClamped` _output_get 6.0 10.0 1.0 7.0))
    (elif (`KismetMathLibrary.InRange_FloatFloat` _output_get 18.0 22.0)
      (`LightComponent.SetIntensity` _lightcomponent (`KismetMathLibrary.MapRangeClamped` _output_get 18.0 22.0 10.0))
      (`SkyLightComponent.SetIntensity` _lightcomponent_2 (`KismetMathLibrary.MapRangeClamped` _output_get 18.0 22.0 7.0 1.0)))))

(fn `SetHowLongDay`
  (params (`Unit : Minute` :type "Float (double-precision)"))
  (set `/Game/OriginalContents/GoodSky/Blueprint/BP_GoodSky.└ How long is a day in the game? ( Unit : Minute )` `Unit : Minute` (`self.Sky`)))

(fn `UserConstructionScript`)