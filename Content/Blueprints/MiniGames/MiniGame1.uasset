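; Actor that hosts the first minigame, whose screen is the MiniGame1_Widget.
; On BeginPlay it creates and displays the widget, sets its IsStart flag and enables input from player controller 0.
; Up, Down, Left and Right key presses and releases set matching input booleans on the widget.
; Tick polls CanDestroy, which is not set in this graph, to destroy the actor and remove the widget.
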(event `Key|Down`
  (params (Key :type "Key Structure"))
  (:`Pressed`
    (bind _asmini_game_1_widget (cast `/Game/Blueprints/MiniGames/MiniGame1_Widget` (stale `self.ReceiveBeginPlay` _returnvalue)))
    (set `/Game/Blueprints/MiniGames/MiniGame1_Widget.downInput` true _asmini_game_1_widget))
  (:`Released`
    (bind _asmini_game_1_widget_2 (cast `/Game/Blueprints/MiniGames/MiniGame1_Widget` (stale `self.ReceiveBeginPlay` _returnvalue)))
    (set `/Game/Blueprints/MiniGames/MiniGame1_Widget.downInput` false _asmini_game_1_widget_2)))

(event `self.ReceiveBeginPlay`
  (bind _returnvalue (`|CreateWidget` "/Game/Blueprints/MiniGames/MiniGame1_Widget.MiniGame1_Widget_C"))
  (`UserWidget.AddToViewport` _returnvalue 0)
  (set `/Game/Blueprints/MiniGames/MiniGame1_Widget.isStart` true _returnvalue)
  (`self.EnableInput` (`GameplayStatics.GetPlayerController` 0)))

(event `Key|Left`
  (params (Key :type "Key Structure"))
  (:`Pressed`
    (bind _asmini_game_1_widget (cast `/Game/Blueprints/MiniGames/MiniGame1_Widget` (stale `self.ReceiveBeginPlay` _returnvalue)))
    (set `/Game/Blueprints/MiniGames/MiniGame1_Widget.leftInput` true _asmini_game_1_widget))
  (:`Released`
    (bind _asmini_game_1_widget_2 (cast `/Game/Blueprints/MiniGames/MiniGame1_Widget` (stale `self.ReceiveBeginPlay` _returnvalue)))
    (set `/Game/Blueprints/MiniGames/MiniGame1_Widget.leftInput` false _asmini_game_1_widget_2)))

(event `Key|Right`
  (params (Key :type "Key Structure"))
  (:`Pressed`
    (bind _asmini_game_1_widget (cast `/Game/Blueprints/MiniGames/MiniGame1_Widget` (stale `self.ReceiveBeginPlay` _returnvalue)))
    (set `/Game/Blueprints/MiniGames/MiniGame1_Widget.rightInput` true _asmini_game_1_widget))
  (:`Released`
    (bind _asmini_game_1_widget_2 (cast `/Game/Blueprints/MiniGames/MiniGame1_Widget` (stale `self.ReceiveBeginPlay` _returnvalue)))
    (set `/Game/Blueprints/MiniGames/MiniGame1_Widget.rightInput` false _asmini_game_1_widget_2)))

(event `self.ReceiveTick`
  (params (DeltaSeconds :type "Float (single-precision)"))
  (if (`self.canDestroy`)
    (`self.K2_DestroyActor`)
    (`Widget.RemoveFromParent` (stale `self.ReceiveBeginPlay` _returnvalue))))

(event `Key|Up`
  (params (Key :type "Key Structure"))
  (:`Pressed`
    (bind _asmini_game_1_widget (cast `/Game/Blueprints/MiniGames/MiniGame1_Widget` (stale `self.ReceiveBeginPlay` _returnvalue)))
    (set `/Game/Blueprints/MiniGames/MiniGame1_Widget.upInput` true _asmini_game_1_widget))
  (:`Released`
    (bind _asmini_game_1_widget_2 (cast `/Game/Blueprints/MiniGames/MiniGame1_Widget` (stale `self.ReceiveBeginPlay` _returnvalue)))
    (set `/Game/Blueprints/MiniGames/MiniGame1_Widget.upInput` false _asmini_game_1_widget_2)))

(fn `UserConstructionScript`)