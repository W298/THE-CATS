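; Patrol NPC that walks a looping route and greets when interacted with at close range.
; From BeginPlay, PatrolPoint runs AIMoveTo toward the current Target actor, then on success advances PatrolNum, wraps at the array's end and calls itself again.
; Interact checks the supplied distance against a threshold, prints the NPC's name and, if the SoundManager cast succeeds, plays a 2D Hello sound.
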(event `/Game/Blueprints/Interface/Interact_Interface.Interact`
  (params (Distance :type "Float (single-precision)"))
  (if (<= Distance 200.0)
    (`KismetSystemLibrary.PrintString` (`KismetStringLibrary.Concat_StrStr` "Interact with " (`KismetSystemLibrary.GetDisplayName` self)))
    (castclass `/Game/Blueprints/Sounds/SoundManager` "/Game/Blueprints/Sounds/SoundManager.SoundManager_C")
    (`GameplayStatics.PlaySound2D` "/Game/Blueprints/Sounds/hello.hello" 1.0 1.0 0.0 null null)))

(event `self.ReceiveBeginPlay`
  (`self.PatrolPoint`))

(event `PatrolPoint`
  (`|AIMoveTo` self (0.0 0.0 0.0) (`|GetArrayItem` (`self.Target`) (`self.PatrolNum`))
    (:`OnSuccess`
      (if (>= (`self.PatrolNum`) (- (`KismetArrayLibrary.Array_Length` (`self.Target`)) 1))
        (set `self.PatrolNum` 0)
        (else
          (`/Engine/EditorBlueprintResources/StandardMacros.IncrementInt` (`self.PatrolNum`)
            (:`  `
              _))))
      (`self.PatrolPoint`))))

(fn `UserConstructionScript`)