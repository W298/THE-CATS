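; Daughter NPC that walks a looping patrol through its Targets and can be talked to by the player.
; BeginPlay starts PatrolPoint, which re-calls itself after each successful AIMoveTo, wrapping the index.
; Interact within range plays a greeting, opens NPC_Interaction_UI and stops the mesh animation, without cancelling the move.
; Tick resumes the animation once FloatingUI is false, though no live logic here clears that flag.
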(event `/Game/Blueprints/Interface/Interact_Interface.Interact`
  (params (Distance :type "Float (single-precision)"))
  (if (<= Distance 200.0)
    (if (not (`self.FloatingUI`))
      (`GameplayStatics.PlaySound2D` "/Game/Blueprints/Sounds/hello.hello" 1.0 1.0 0.0 null null)
      (bind _returnvalue (`|CreateWidget` "/Game/Blueprints/UI/NPC_Interaction_UI.NPC_Interaction_UI_C"))
      (`UserWidget.AddToViewport` _returnvalue 0)
      (set `self.floatingUI` true)
      (`SkeletalMeshComponent.Stop` (`self.Mesh`))
      (set `self.IsStop` true))))

(event `self.ReceiveTick`
  (params (DeltaSeconds :type "Float (single-precision)"))
  (if (`self.IsStop`)
    (if (not (`self.FloatingUI`))
      (`SkeletalMeshComponent.Play` (`self.Mesh`) false)
      (set `self.IsStop` false))))

(event `self.ReceiveBeginPlay`
  (`self.PatrolPoint`))

(event `PatrolPoint`
  (`|AIMoveTo` self (0.0 0.0 0.0) (`|GetArrayItem` (`self.Targets`) (`self.PatrolNum`))
    (:`OnSuccess`
      (if (>= (`self.PatrolNum`) (- (`KismetArrayLibrary.Array_Length` (`self.Targets`)) 1))
        (set `self.PatrolNum` 0)
        (else
          (`/Engine/EditorBlueprintResources/StandardMacros.IncrementInt` (`self.PatrolNum`)
            (:`  `
              _))))
      (`self.PatrolPoint`))))

(fn `UserConstructionScript`)