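; Mother2 is a patrolling NPC that opens an interaction widget when interacted with at close range.
; It loops through Targets until the game mode's time passes 18, then walks Home and destroys itself.
; Interaction halts it and sets the game instance's NPC index; Tick removes the widget on left click and resumes patrol.
; Tick also loads the cat house ending once Favorability and Reputation both reach 100.
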(event `/Game/Blueprints/Interface/Interact_Interface.Interact`
  (params (Distance :type "Float (single-precision)"))
  (if (<= Distance 200.0)
    (if (not (`self.FloatingUI`))
      (`GameplayStatics.PlaySound2D` "/Game/Blueprints/Sounds/hello.hello" 1.0 1.0 0.0 null null)
      (bind _returnvalue (`|CreateWidget` "/Game/Blueprints/UI/NPC_Interaction_UI.NPC_Interaction_UI_C"))
      (`UserWidget.AddToViewport` _returnvalue 0)
      (set `self.floatingUI` true)
      (`SkeletalMeshComponent.Stop` (`self.Mesh`))
      (set `self.IsStop` true)
      (`NavMovementComponent.StopActiveMovement` (`self.CharacterMovement`))
      (bind _asplayer_cat (cast `/Game/Blueprints/Player/Player_Cat` (`GameplayStatics.GetPlayerPawn` 0)))
      (set `/Game/Blueprints/Player/Player_Cat.ShowUI` false _asplayer_cat)
      (bind _asgame_ins (cast `/Game/Blueprints/GameMode/GameIns` (`GameplayStatics.GetGameInstance`)))
      (set `/Game/Blueprints/GameMode/GameIns.npc_index` 4 _asgame_ins))))

(event `self.ReceiveTick`
  (params (DeltaSeconds :type "Float (single-precision)"))
  (if (and (>= (`self.Favorability`) 100) (>= (`self.Reputation`) 100))
    (`GameplayStatics.OpenLevel` "Ending_Cat_House")
    (elif (`self.IsStop`)
      (if (`self.FloatingUI`)
        (`KismetSystemLibrary.Delay` 0.2)
        (bind _asplayer_cat (cast `/Game/Blueprints/Player/Player_Cat` (`GameplayStatics.GetPlayerPawn` 0)))
        (if (`/Game/Blueprints/Player/Player_Cat.onLeftMouseClick` _asplayer_cat)
          (if (`self.floatingUI`)
            (`Widget.RemoveFromParent` (stale `/Game/Blueprints/Interface/Interact_Interface.Interact` _returnvalue))
            (set `self.FloatingUI` false)))
        (else
          (`SkeletalMeshComponent.Play` (`self.Mesh`) true)
          (set `self.IsStop` false)
          (`self.PatrolPoint`))))))

(event `self.ReceiveBeginPlay`
  (`self.PatrolPoint`))

(event `PatrolPoint`
  (bind _asmain_gm (cast `/Game/Blueprints/GameMode/Main_GM` (`GameplayStatics.GetGameMode`)))
  (if (<= (`/Game/Blueprints/GameMode/Main_GM.CurrentTime` _asmain_gm) 18.0)
    (`|AIMoveTo` self (0.0 0.0 0.0) (`|GetArrayItem` (`self.Targets`) (`self.PatrolNum`))
      (:`OnSuccess`
        (if (>= (`self.PatrolNum`) (- (`KismetArrayLibrary.Array_Length` (`self.Targets`)) 1))
          (set `self.PatrolNum` 0)
          (else
            (`/Engine/EditorBlueprintResources/StandardMacros.IncrementInt` (`self.PatrolNum`)
              (:`  `
                _))))
        (`self.PatrolPoint`)))
    (else
      (`|AIMoveTo` null (0.0 0.0 0.0) (`self.Home`)
        (:`OnSuccess`
          (`self.K2_DestroyActor`))))))

(fn `UserConstructionScript`)