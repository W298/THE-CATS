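; Traffic path actor that spawns random vehicles to drive along its spline.
; On BeginPlay it spawns one vehicle, then loops every two seconds with a one-in-eleven chance of spawning another.
; SpawnCar picks one of eight vehicle classes, from bus to truck, and places it at the first spline point.
; Each vehicle receives the spline and Reverse flag through SetPath, then starts with Run.
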(event `self.ReceiveBeginPlay`
  (`self.SpawnCar`)
  (if (== (`KismetMathLibrary.RandomIntegerInRange` 0 10) 0) :!label _label
    (`self.SpawnCar`))
  (`KismetSystemLibrary.Delay` 2.0)
  (goto _label))

(event `SpawnCar`
  (bind _car (`self.Car`))
  (bind _returnvalue (`KismetMathLibrary.MakeTransform` (`SplineComponent.GetLocationAtSplinePoint` (`self.Spline`) 0 "World")))
  (switch `int` (`KismetMathLibrary.RandomIntegerInRange` 0 7)
    (:`0`
      (bind _returnvalue_2 (`|SpawnActorFromClass` "/Game/Blueprints/Car/Bus.Bus_C" _returnvalue "Undefined" "OverrideRootScale" null null))
      (set `self.Car` _returnvalue_2))
    (:`1`
      (bind _returnvalue_3 (`|SpawnActorFromClass` "/Game/Blueprints/Car/Car.Car_C" _returnvalue "Undefined" "OverrideRootScale" null null))
      (set `self.Car` _returnvalue_3))
    (:`2`
      (bind _returnvalue_4 (`|SpawnActorFromClass` "/Game/Blueprints/Car/DeliveryTruck.DeliveryTruck_C" _returnvalue "Undefined" "OverrideRootScale" null null))
      (set `self.Car` _returnvalue_4))
    (:`3`
      (bind _returnvalue_5 (`|SpawnActorFromClass` "/Game/Blueprints/Car/Firetruck.Firetruck_C" _returnvalue "Undefined" "OverrideRootScale" null null))
      (set `self.Car` _returnvalue_5))
    (:`4`
      (bind _returnvalue_6 (`|SpawnActorFromClass` "/Game/Blueprints/Car/GarbageTruck.GarbageTruck_C" _returnvalue "Undefined" "OverrideRootScale" null null))
      (set `self.Car` _returnvalue_6))
    (:`5`
      (bind _returnvalue_7 (`|SpawnActorFromClass` "/Game/Blueprints/Car/Pickup.Pickup_C" _returnvalue "Undefined" "OverrideRootScale" null null))
      (set `self.Car` _returnvalue_7))
    (:`6`
      (bind _returnvalue_8 (`|SpawnActorFromClass` "/Game/Blueprints/Car/SchoolBus.SchoolBus_C" _returnvalue "Undefined" "OverrideRootScale" null null))
      (set `self.Car` _returnvalue_8))
    (:`7`
      (bind _returnvalue_9 (`|SpawnActorFromClass` "/Game/Blueprints/Car/Truck.Truck_C" _returnvalue "Undefined" "OverrideRootScale" null null))
      (set `self.Car` _returnvalue_9)))
  (`/Game/Blueprints/Car/Vehicle.SetPath` _car (`self.Spline`) (`self.Reverse`))
  (`/Game/Blueprints/Car/Vehicle.Run` _car))

(fn `UserConstructionScript`)