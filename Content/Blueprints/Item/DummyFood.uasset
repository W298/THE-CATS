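; Edible food item that applies a good, moderate or harmful effect to the player when eaten at close range.
; On Interact within range, FoodKindDecision maps actor tags to food kinds, then after a short delay the item flags Eat and destroys itself.
; FoodKind groups kinds into three tiers, setting FoodState and adding an Effecter to the player pawn that changes health, hunger, fatigue and max stamina.
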(event `/Game/Blueprints/Interface/Interact_Interface.Interact`
  (params (Distance :type "Float (single-precision)"))
  (if (<= Distance 100.0)
    (`self.Food Kind Decision`)
    (`KismetSystemLibrary.Delay` 1.0)
    (set `self.Eat` true)
    (`self.K2_DestroyActor`)
    (`KismetSystemLibrary.PrintString` (`KismetStringLibrary.Concat_StrStr` "Interact with " (`KismetSystemLibrary.GetDisplayName` self)))))

(fn `Food Kind Decision`
  (bind _tags (`self.Tags`))
  (`|ExecutionSequence`
    (:`then_0`
      (if (`KismetArrayLibrary.Array_Contains` _tags "EatFruit")
        (`self.FoodKind` "NewEnumerator7")
        (`KismetSystemLibrary.PrintString` "Fruits")))
    (:`then_1`
      (if (`KismetArrayLibrary.Array_Contains` _tags "Fish")
        (`self.FoodKind` "NewEnumerator0")
        (`KismetSystemLibrary.PrintString` "Fish")))
    (:`then_2`
      (if (`KismetArrayLibrary.Array_Contains` _tags "Chocolate")
        (`self.FoodKind` "NewEnumerator10")
        (`KismetSystemLibrary.PrintString` "Cake")))
    (:`then_3`
      (if (`KismetArrayLibrary.Array_Contains` _tags "Rat")
        (`self.FoodKind` "NewEnumerator1")))
    (:`then_4`
      (if (`KismetArrayLibrary.Array_Contains` _tags "Bug")
        (`self.FoodKind` "NewEnumerator2")))
    (:`then_5`
      (if (`KismetArrayLibrary.Array_Contains` _tags "CatFeed")
        (`self.FoodKind` "NewEnumerator4")))
    (:`then_6`
      (if (`KismetArrayLibrary.Array_Contains` _tags "LeftOver")
        (`self.FoodKind` "NewEnumerator5")))
    (:`then_7`
      (if (`KismetArrayLibrary.Array_Contains` _tags "Vegetable")
        (`self.FoodKind` "NewEnumerator6")))
    (:`then_8`
      (if (`KismetArrayLibrary.Array_Contains` _tags "DangerFruit")
        (`self.FoodKind` "NewEnumerator8")))
    (:`then_9`
      (if (`KismetArrayLibrary.Array_Contains` _tags "Mlik")
        (`self.FoodKind` "NewEnumerator9")))
    (:`then_10`
      (if (`KismetArrayLibrary.Array_Contains` _tags "Garlic")
        (`self.FoodKind` "NewEnumerator11")))
    (:`then_11`
      (if (`KismetArrayLibrary.Array_Contains` _tags "Onion")
        (`self.FoodKind` "NewEnumerator12")))))

(fn `FoodKind`
  (params (FoodKind :type "/Game/Blueprints/Item/Food_Kind__Enum Enum" :default "NewEnumerator0"))
  (switch `/Game/Blueprints/Item/Food_Kind__Enum` FoodKind
    (:`NewEnumerator0`
      (set `self.FoodState` "NewEnumerator0" :!label _label)
      (bind _returnvalue (`AddComponent|NODE_AddEffecter-0` :`self` (`GameplayStatics.GetPlayerPawn` 0)))
      (`/Game/Blueprints/Player/Effecter.Custom Effect` _returnvalue 5.0 10.0 2.0 0.0 0.0 1.0 true 5.0 false false false false false))
    (:`NewEnumerator1`
      (goto _label))
    (:`NewEnumerator2`
      (goto _label))
    (:`NewEnumerator3`
      (goto _label))
    (:`NewEnumerator4`
      (goto _label))
    (:`NewEnumerator5`
      (set `self.FoodState` "NewEnumerator1" :!label _label_2)
      (bind _returnvalue_2 (`AddComponent|NODE_AddEffecter-1` :`self` (`GameplayStatics.GetPlayerPawn` 0)))
      (`/Game/Blueprints/Player/Effecter.Custom Effect` _returnvalue_2 3.0 4.0 3.0 0.0 0.0 1.0 true 3.0 false false false false false))
    (:`NewEnumerator6`
      (goto _label_2))
    (:`NewEnumerator7`
      (goto _label_2))
    (:`NewEnumerator8`
      (set `self.FoodState` "NewEnumerator2" :!label _label_3)
      (bind _returnvalue_3 (`AddComponent|NODE_AddEffecter-2` :`self` (`GameplayStatics.GetPlayerPawn` 0)))
      (`/Game/Blueprints/Player/Effecter.Custom Effect` _returnvalue_3 -4.0 -2.0 4.0 0.0 0.0 1.0 true -4.0 false false false false false))
    (:`NewEnumerator9`
      (goto _label_3))
    (:`NewEnumerator10`
      (goto _label_3))
    (:`NewEnumerator11`
      (goto _label_3))
    (:`NewEnumerator12`
      (goto _label_3))))

(fn `UserConstructionScript`)