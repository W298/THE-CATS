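; Cat spawn-point actor that places an AI-controlled Other_Cat at its own location when play begins.
; On BeginPlay it casts the game mode to Main_GM, stores it and aborts if the cast fails.
; It then spawns the cat with zero rotation, gives it a default controller and randomly swaps its skeletal mesh to one of five low-poly kitten variants.
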(event `self.ReceiveBeginPlay`
  (bind _asmain_gm (cast `/Game/Blueprints/GameMode/Main_GM` (`GameplayStatics.GetGameMode`)))
  (set `self.GM` _asmain_gm)
  (bind _returnvalue (`|SpawnActorFromClass` "/Game/Blueprints/Player/Other_Cat.Other_Cat_C" (`KismetMathLibrary.MakeTransform` (`self.K2_GetActorLocation`)) "AdjustIfPossibleButAlwaysSpawn" "OverrideRootScale" null null))
  (`Pawn.SpawnDefaultController` _returnvalue)
  (switch `int` (`KismetMathLibrary.RandomIntegerInRange` 0 4)
    (:`0`
      (bind _mesh (`Character.Mesh` _returnvalue))
      (`SkinnedMeshComponent.SetSkinnedAssetAndUpdate` _mesh "/Game/OriginalContents/LowPoly_Kitten/Meshes/Mesh_LowPoly_Kitten_Abyss.Mesh_LowPoly_Kitten_Abyss" true))
    (:`1`
      (`SkinnedMeshComponent.SetSkinnedAssetAndUpdate` _mesh "/Game/OriginalContents/LowPoly_Kitten/Meshes/Mesh_LowPoly_Kitten_Black.Mesh_LowPoly_Kitten_Black" true))
    (:`2`
      (`SkinnedMeshComponent.SetSkinnedAssetAndUpdate` _mesh "/Game/OriginalContents/LowPoly_Kitten/Meshes/Mesh_LowPoly_Kitten_BlWt.Mesh_LowPoly_Kitten_BlWt" true))
    (:`3`
      (`SkinnedMeshComponent.SetSkinnedAssetAndUpdate` _mesh "/Game/OriginalContents/LowPoly_Kitten/Meshes/Mesh_LowPoly_Kitten_Maine.Mesh_LowPoly_Kitten_Maine" true))
    (:`4`
      (`SkinnedMeshComponent.SetSkinnedAssetAndUpdate` _mesh "/Game/OriginalContents/LowPoly_Kitten/Meshes/Mesh_LowPoly_Kitten_White.Mesh_LowPoly_Kitten_White" true))))

(fn `UserConstructionScript`)