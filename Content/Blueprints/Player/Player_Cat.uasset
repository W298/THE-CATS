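; Player cat character with mouse-aimed movement, survival stats and click interaction.
; Each tick it yaws toward the cursor's ground-plane projection, eases spring-arm zoom and checks hunger to toggle starvation.
; Forward-only input is interpolated to drive walk speed, with sprint draining stamina through an effecter and exhaustion halving speed.
; Left click traces from the camera and sends an interact message with distance; F enables hypothermia, and optional gizmos show debug info.
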(event `self.ReceiveBeginPlay`
  (set `PlayerController.bShowMouseCursor` true (`GameplayStatics.GetPlayerController` 0)))

(event `self.ReceiveTick`
  (params (DeltaSeconds :type "Float (single-precision)"))
  (`self.SetRotation`)
  (`self.ZoomTick`)
  (`self.DebugStatusValue`)
  (`self.CheckStarvation`))

(event `Key|F`
  (params (Key :type "Key Structure"))
  (:`Pressed`
    (bind _returnvalue (`AddComponent|NODE_AddEffecter-6`))
    (`/Game/Blueprints/Player/Effecter.Enable Hypothermia` _returnvalue)))

(event `InputAxis|MoveForward`
  (params (AxisValue :type "Float (single-precision)"))
  (bind _returnvalue (`KismetMathLibrary.FInterpTo` (`self.FrontAxisValue`) (`KismetMathLibrary.FClamp` AxisValue 0.0 (`self.MaxFrontAxisValue`)) (`GameplayStatics.GetWorldDeltaSeconds`) 3.0))
  (bind _value (`self.Get Status Value` "NewEnumerator3"))
  (if (not (> _value 0.0))
    (set `self.MaxFrontAxisValue` (/ (`self.DefaultMaxFrontAxisValue`) 2.0))
    (`self.Set Behavior Value` "NewEnumerator0"))
  (`self.AddMovementInput` (`self.GetActorForwardVector`) _returnvalue)
  (bind _output_get (set `self.FrontAxisValue` _returnvalue))
  (set `CharacterMovementComponent.MaxWalkSpeed` (`KismetMathLibrary.MapRangeUnclamped` _output_get 0.0 1.0 0.0 180.0) (`self.CharacterMovement`)))

(event `InputAction|Jump`
  (params (Key :type "Key Structure"))
  (:`Pressed`
    (`self.Jump`)))

(event `InputAction|Sprint`
  (params (Key :type "Key Structure"))
  (bind _defaultmaxfrontaxisvalue (`self.DefaultMaxFrontAxisValue`))
  (bind _effecter_gerneral (`self.Effecter_Gerneral`))
  (:`Pressed`
    (set `self.MaxFrontAxisValue` _defaultmaxfrontaxisvalue)
    (`self.Set Behavior Value` "NewEnumerator0" true)
    (`/Game/Blueprints/Player/Effecter_Gerneral.StartDecreaseStamina` _effecter_gerneral))
  (:`Released`
    (set `self.MaxFrontAxisValue` (/ _defaultmaxfrontaxisvalue 2.0))
    (`self.Set Behavior Value` "NewEnumerator0")
    (`/Game/Blueprints/Player/Effecter_Gerneral.StopDecreaseStamina` _effecter_gerneral)))

(event `ZoomTick`
  (bind _targetarmlength (`SpringArmComponent.TargetArmLength` (`self.SpringArm`)))
  (if (not (`KismetMathLibrary.NearlyEqual_FloatFloat` _targetarmlength (`self.DesireZoom`) 0.001))
    (set `SpringArmComponent.TargetArmLength` (`KismetMathLibrary.Lerp` _targetarmlength (`self.DesireZoom`) (* (`self.ZoomSpeed`) (`GameplayStatics.GetWorldDeltaSeconds`))) (`self.SpringArm`))))

(event `Key|MouseScrollUp`
  (params (Key :type "Key Structure"))
  (:`Pressed`
    (set `self.DesireZoom` (`KismetMathLibrary.FClamp` (+ (`SpringArmComponent.TargetArmLength` (`self.SpringArm`)) -300.0) (`self.MinZoom`) (`self.MaxZoom`)))))

(event `Key|MouseScrollDown`
  (params (Key :type "Key Structure"))
  (:`Pressed`
    (set `self.DesireZoom` (`KismetMathLibrary.FClamp` (+ (`SpringArmComponent.TargetArmLength` (`self.SpringArm`)) 300.0) (`self.MinZoom`) (`self.MaxZoom`)))))

(event `Key|LeftMouseButton`
  (params (Key :type "Key Structure"))
  (bind _returnvalue (`SceneComponent.K2_GetComponentLocation` (`self.Camera`)))
  (:`Pressed`
    (bind _outhit (`KismetSystemLibrary.LineTraceSingle` _returnvalue (* (- (`self.MousePosition`) _returnvalue) 10000) "TraceTypeQuery2"))
    (bind (_bblockinghit _binitialoverlap _time _distance _location _impactpoint _normal _impactnormal _physmat _hitactor) (`GameplayStatics.BreakHitResult` _outhit))
    (`self.DebugInteract` _hitactor)
    (message `/Game/Blueprints/Interface/Interact_Interface.Interact` _hitactor (`KismetMathLibrary.Vector_Distance` (`self.K2_GetActorLocation` _hitactor) (`self.K2_GetActorLocation`)))))

(fn `CheckStarvation`
  (bind _value (`self.Get Status Value` "NewEnumerator1"))
  (if (<= _value 0.0)
    (bind _returnvalue (`AddComponent|NODE_AddEffecter-4`))
    (`/Game/Blueprints/Player/Effecter.Enable Starvation` _returnvalue)
    (set `self.isStarving` true)
    (elif (`self.isStarving`)
      (`/Game/Blueprints/Player/Effecter.Disable Starvation` _returnvalue)
      (set `self.isStarving` false))))

(fn `DebugInteract`
  (params (Object :type "Actor Object Reference"))
  (bind _returnvalue (`self.K2_GetActorLocation` Object))
  (bind _returnvalue_2 (`self.K2_GetActorLocation`))
  (if (`self.DebugGizmoOn`)
    (`KismetSystemLibrary.DrawDebugLine` _returnvalue _returnvalue_2 (struct :`R` 1.0 :`B` 0.847059 :`A` 1.0) 1.0 1.0)
    (`KismetSystemLibrary.DrawDebugString` _returnvalue (`KismetSystemLibrary.GetDisplayName` Object) null (struct :`R` 1.0 :`B` 0.847059 :`A` 1.0) 1.0)
    (`KismetSystemLibrary.DrawDebugString` (/ (+ _returnvalue _returnvalue_2) 2) (`KismetStringLibrary.Conv_DoubleToString` (`KismetMathLibrary.Vector_Distance` _returnvalue_2 _returnvalue)) null (struct :`R` 1.0 :`B` 0.847059 :`A` 1.0) 1.0)))

(fn `DebugStatusValue`
  (bind (_health _hunger _fatigue _stamina) (break `/Game/Blueprints/Player/Player_StatusValue` (`self.StatusValue`)))
  (if (`self.DebugGizmoOn`)
    (`KismetSystemLibrary.DrawDebugString` (`self.K2_GetActorLocation`) (`KismetStringLibrary.Concat_StrStr` (`KismetStringLibrary.Concat_StrStr` "Health : " (`KismetStringLibrary.Conv_DoubleToString` _health) " \n") (`KismetStringLibrary.Concat_StrStr` "Hunger : " (`KismetStringLibrary.Conv_DoubleToString` _hunger) " \n") (`KismetStringLibrary.Concat_StrStr` "Fatugue : " (`KismetStringLibrary.Conv_DoubleToString` _fatigue) " \n") (`KismetStringLibrary.Concat_StrStr` "Stamina : " (`KismetStringLibrary.Conv_DoubleToString` _stamina) " \n") (`KismetStringLibrary.Concat_StrStr` "Speed : " (`KismetStringLibrary.Conv_DoubleToString` (`self.MaxFrontAxisValue`)) " \n")) null (struct :`G` 1.0 :`B` 0.190055 :`A` 1.0))))

(fn `Get Behavior Value`
  (params (Target :type "/Game/Blueprints/Player/Player_BehaviorName Enum" :default "NewEnumerator0"))
  (returns (NewParam :type Boolean))
  (switch `/Game/Blueprints/Player/Player_BehaviorName` Target
    (:`NewEnumerator0`
      (return (`.IsSprinting_1_31CCE2FB487F9FD15E718CAB02051BF4` (break `/Game/Blueprints/Player/Player_Behavior` (`self.Behavior`)))))))

(fn `Get Status Value`
  (params (Target :type "/Game/Blueprints/Player/Player_StatusName Enum" :default "NewEnumerator0"))
  (returns (Value :type "Float (double-precision)"))
  (bind (_health _hunger _fatigue _stamina _maxstamina) (break `/Game/Blueprints/Player/Player_StatusValue` (`self.StatusValue`)))
  (switch `/Game/Blueprints/Player/Player_StatusName` Target
    (:`NewEnumerator0`
      (return _health))
    (:`NewEnumerator1`
      (return _hunger))
    (:`NewEnumerator2`
      (return _fatigue))
    (:`NewEnumerator3`
      (return _stamina))
    (:`NewEnumerator4`
      (return _maxstamina))))

(fn `GetLookingPosition`
  (params (Zoffset :type "Float (double-precision)"))
  (returns (MousePos :type "Vector Structure"))
  (bind (_worldlocation _worlddirection) (`PlayerController.DeprojectMousePositionToWorld` (`GameplayStatics.GetPlayerController` 0)))
  (bind _returnvalue (+ _worldlocation (* (* _worlddirection (/ (.z _worldlocation) (.z _worlddirection))) -1.0)))
  (set `self.LookingAtPosition` (+ _returnvalue (`KismetMathLibrary.MakeVector` 0.0 0.0 Zoffset)))
  (return _returnvalue))

(fn `Set Behavior Value`
  (params (Target :type "/Game/Blueprints/Player/Player_BehaviorName Enum" :default "NewEnumerator0") (Value :type Boolean))
  (switch `/Game/Blueprints/Player/Player_BehaviorName` Target
    (:`NewEnumerator0`
      (setmembers `/Game/Blueprints/Player/Player_Behavior` :`StructRef` (`self.Behavior`) :`IsSprinting` Value))))

(fn `Set Max Speed`
  (params (Target :type "Float (double-precision)"))
  (bind _output_get (set `self.DefaultMaxFrontAxisValue` Target))
  (set `self.MaxFrontAxisValue` (/ _output_get 2.0)))

(fn `Set Status Value`
  (params (Target :type "/Game/Blueprints/Player/Player_StatusName Enum" :default "NewEnumerator0") (Value :type "Float (double-precision)"))
  (bind _statusvalue (`self.StatusValue`))
  (switch `/Game/Blueprints/Player/Player_StatusName` Target
    (:`NewEnumerator0`
      (setmembers `/Game/Blueprints/Player/Player_StatusValue` :`StructRef` _statusvalue :`Health` Value))
    (:`NewEnumerator1`
      (setmembers `/Game/Blueprints/Player/Player_StatusValue` :`StructRef` _statusvalue :`Hunger` Value))
    (:`NewEnumerator2`
      (setmembers `/Game/Blueprints/Player/Player_StatusValue` :`StructRef` _statusvalue :`Fatigue` Value))
    (:`NewEnumerator3`
      (setmembers `/Game/Blueprints/Player/Player_StatusValue` :`StructRef` _statusvalue :`Stamina` Value))
    (:`NewEnumerator4`
      (setmembers `/Game/Blueprints/Player/Player_StatusValue` :`StructRef` _statusvalue :`MaxStamina` Value))))

(fn `SetRotation`
  (bind _mousepos (`self.GetLookingPosition` 40.0))
  (set `self.MousePosition` _mousepos)
  (`self.K2_SetActorRelativeRotation` (`KismetMathLibrary.MakeRotator` 0.0 0.0 (.yaw (`KismetMathLibrary.FindLookAtRotation` (`self.K2_GetActorLocation`) (`self.LookingAtPosition`))))))

(fn `UserConstructionScript`)