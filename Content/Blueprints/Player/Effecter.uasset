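; Effecter is a component on Player_Cat that updates the cat's stamina, hunger and fatigue over time.
; It ticks every 0.1 seconds, applying per-stat speeds to the owner's StatusValue struct, clamped to 0–100.
; Start and stop events set a flag that flips the sign of the stamina change.
; Starting also doubles the hunger rate, and stopping resets it to a hardcoded value.
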(event `self.ReceiveBeginPlay`
  (`self.SetComponentTickInterval` 0.1)
  (bind _asplayer_cat (cast `/Game/Blueprints/Player/Player_Cat` (`self.GetOwner`)))
  (set `self.Target` _asplayer_cat))

(event `self.ReceiveTick`
  (params (DeltaSeconds :type "Float (single-precision)"))
  (`self.DecreaseStamina` (`self.StaminaSpeed`))
  (`self.DecreaseHunger` (`self.HungerSpeed`))
  (`self.IncreaseFatigue` (`self.FatigueSpeed`)))

(event `StartDecreaseStamina`
  (set `self.IsDecreasingStamina` true)
  (set `self.HungerSpeed` (* 2 (`self.HungerSpeed`))))

(event `StopDecreaseStamina`
  (set `self.IsDecreasingStamina` false)
  (set `self.HungerSpeed` -0.016667))

(fn `DecreaseHunger`
  (params (Unit :type "Float (double-precision)"))
  (bind _statusvalue (`/Game/Blueprints/Player/Player_Cat.StatusValue` (`self.Target`)))
  (setmembers `/Game/Blueprints/Player/Player_StatusValue` :`StructRef` _statusvalue :`Hunger` (`KismetMathLibrary.FClamp` (+ (`.Hunger_5_6D6A959D422A59C377099080C08CD485` (break `/Game/Blueprints/Player/Player_StatusValue` _statusvalue)) Unit) 0.0 100.0)))

(fn `DecreaseStamina`
  (params (Unit :type "Float (double-precision)"))
  (bind _statusvalue (`/Game/Blueprints/Player/Player_Cat.StatusValue` (`self.Target`)))
  (bind ((`Stamina_9_0D14C794493D9EFB251AF7990E2805A0` _stamina)) (break `/Game/Blueprints/Player/Player_StatusValue` _statusvalue))
  (if (`self.IsDecreasingStamina`)
    (setmembers `/Game/Blueprints/Player/Player_StatusValue` :`StructRef` _statusvalue :`Stamina` (`KismetMathLibrary.FClamp` (+ _stamina Unit) 0.0 100.0))
    (else
      (setmembers `/Game/Blueprints/Player/Player_StatusValue` :`StructRef` _statusvalue :`Stamina` (`KismetMathLibrary.FClamp` (- _stamina Unit) 0.0 100.0)))))

(fn `IncreaseFatigue`
  (params (Unit :type "Float (double-precision)"))
  (bind _statusvalue (`/Game/Blueprints/Player/Player_Cat.StatusValue` (`self.Target`)))
  (setmembers `/Game/Blueprints/Player/Player_StatusValue` :`StructRef` _statusvalue :`Fatigue` (`KismetMathLibrary.FClamp` (+ (`.Fatigue_7_563C97174B5D06BA9C9355BEC07BDD90` (break `/Game/Blueprints/Player/Player_StatusValue` _statusvalue)) Unit) 0.0 100.0)))