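; Player status component for Player_Cat that continuously changes stamina, hunger, fatigue and health over time.
; It ticks every 0.1 seconds, adding a per-stat speed clamped between zero and that stat's maximum.
; Sprint events switch the stamina and hunger rates, with sprint start gated by AutoReduceStamina.
; AutoRecoverStamina gates only non-negative stamina changes, while AutoRecoverHealth gates all health changes, which go through the owner's SetStatusValue.
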(event `self.ReceiveBeginPlay`
  (`self.SetComponentTickInterval` 0.1)
  (bind _asplayer_cat (cast `/Game/Blueprints/Player/Player_Cat` (`self.GetOwner`)))
  (set `self.Target` _asplayer_cat))

(event `self.ReceiveTick`
  (params (DeltaSeconds :type "Float (single-precision)"))
  (`self.AddStamina` (`self.StaminaAddSpeed`))
  (`self.AddHunger` (`self.HungerAddSpeed`))
  (`self.AddFatigue` (`self.FatigueAddSpeed`))
  (`self.AddHealth` (`self.HealthAddSpeed`)))

(event `StartSprint`
  (if (`self.AutoReduceStamina`)
    (set `self.StaminaAddSpeed` (`self.DefaultStaminaAddSpeed`))
    (set `self.HungerAddSpeed` (* 2 (`self.DefaultHungerAddSpeed`)))))

(event `EndSprint`
  (set `self.StaminaAddSpeed` (* -1 (`self.DefaultStaminaAddSpeed`)))
  (set `self.HungerAddSpeed` (`self.DefaultHungerAddSpeed`)))

(fn `AddFatigue`
  (params (Unit :type "Float (double-precision)"))
  (bind _statusvalue (`/Game/Blueprints/Player/Player_Cat.StatusValue` (`self.Target`)))
  (bind ((`Fatigue_7_563C97174B5D06BA9C9355BEC07BDD90` _fatigue) (`MaxFatigue_21_E53FCBFF4F19334DEFB5B697D6DC5680` _maxfatigue)) (break `/Game/Blueprints/Player/Player_StatusValue` _statusvalue))
  (setmembers `/Game/Blueprints/Player/Player_StatusValue` :`StructRef` _statusvalue :`Fatigue` (`KismetMathLibrary.FClamp` (+ _fatigue Unit) 0.0 _maxfatigue)))

(fn `AddHealth`
  (params (Unit :type "Float (double-precision)"))
  (bind _target (`self.Target`))
  (bind ((`Health_2_FEC5E8B949E1CBB1341517B96C258ED1` _health) (`MaxHealth_18_A747FC1A4F465DFDAAC4239C8E8D162D` _maxhealth)) (break `/Game/Blueprints/Player/Player_StatusValue` (`/Game/Blueprints/Player/Player_Cat.StatusValue` _target)))
  (if (`self.AutoRecoverHealth`)
    (`/Game/Blueprints/Player/Player_Cat.Set Status Value` _target "NewEnumerator0" (`KismetMathLibrary.FClamp` (+ _health Unit) 0.0 _maxhealth))))

(fn `AddHunger`
  (params (Unit :type "Float (double-precision)"))
  (bind _statusvalue (`/Game/Blueprints/Player/Player_Cat.StatusValue` (`self.Target`)))
  (bind ((`Hunger_5_6D6A959D422A59C377099080C08CD485` _hunger) (`MaxHunger_19_70124C6D48C06B509E6784959DF2314B` _maxhunger)) (break `/Game/Blueprints/Player/Player_StatusValue` _statusvalue))
  (setmembers `/Game/Blueprints/Player/Player_StatusValue` :`StructRef` _statusvalue :`Hunger` (`KismetMathLibrary.FClamp` (+ _hunger Unit) 0.0 _maxhunger)))

(fn `AddStamina`
  (params (Unit :type "Float (double-precision)"))
  (bind _statusvalue (`/Game/Blueprints/Player/Player_Cat.StatusValue` (`self.Target`)))
  (bind ((`Stamina_9_0D14C794493D9EFB251AF7990E2805A0` _stamina) (`MaxStamina_12_A7D63900478D92A473C4ED992477968F` _maxstamina)) (break `/Game/Blueprints/Player/Player_StatusValue` _statusvalue))
  (if (< Unit 0.0)
    (setmembers `/Game/Blueprints/Player/Player_StatusValue` :`StructRef` _statusvalue :`Stamina` (`KismetMathLibrary.FClamp` (+ _stamina Unit) 0.0 _maxstamina) :!label _label)
    (elif (`self.AutoRecoverStamina`)
      (goto _label))))